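; Manager actor for a search-and-find minigame built around audio clues from a Rounds array.
; StartGame shows the WBP_ObjectsGame widget and mouse cursor and hides the crosshair.
; CheckAnswer tests the clicked actor's tag, then plays a wrong sound, ends the game or plays the next clue after a delay.
; Logic is unfinished: the tag is "None", the round increment is unwired, and the completion comparison looks inverted.
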(event Custom|StartGame
  (bind _returnvalue (Game|GetPlayerController 0))
  (Variables|Default|SetbGameActive true)
  (Development|PrintString "Hello")
  (Variables|Default|SetCurrentRoundIndex 0)
  (bind _returnvalue_2 (UserInterface|CreateWidget "/Game/Events/WBP_ObjectsGame.WBP_ObjectsGame_C"))
  (UserInterface|Viewport|AddtoViewport _returnvalue_2 0)
  (Variables|/Script/Engine.PlayerController|SetbShowMouseCursor _returnvalue true)
  (bind _foundwidgets (Widget|GetAllWidgetsOfClass "/Game/Events/WBP_Crosshair.WBP_Crosshair_C" true))
  (Widget|SetVisibility (Utilities|Array|Get(acopy) _foundwidgets) "Hidden")
  (Input|SetInputModeGameandUI _returnvalue 0 "DoNotLock" true false))

(event Custom|PlayCurrentClue
  (Audio|PlaySound2D (.AudioClue (Utilities|Struct|BreakS_SearchRound (Utilities|Array|Get(acopy) (Variables|Default|GetRounds) (Variables|Default|GetCurrentRoundIndex)))) 1.0 1.0 0.0 0 0))

(event Custom|CheckAnswer
  (params (ClickedActor :type Actor%20Object%20Reference))
  (bind _returnvalue (Game|GetPlayerController 0))
  (if (Actor|ActorHasTag ClickedActor "None")
    (Variables|Default|SetCurrentRoundIndex (stale _result))
    (if (<= (Variables|Default|GetCurrentRoundIndex) (Utilities|Array|Length (Variables|Default|GetRounds)))
      (Audio|PlaySound2D (Variables|Default|GetSFX_Complete) 1.0 1.0 0.0 0 0)
      (Variables|Default|SetbGameActive false)
      (Variables|/Script/Engine.PlayerController|SetbShowMouseCursor _returnvalue false)
      (bind _foundwidgets (Widget|GetAllWidgetsOfClass 0 true))
      (Widget|SetVisibility (Utilities|Array|Get(acopy) _foundwidgets) "Visible")
      (Input|SetInputModeGameOnly _returnvalue false)
      (else
        (Utilities|FlowControl|Delay 1.5)
        (CallFunction|PlayCurrentClue)))
    (else
      (Audio|PlaySound2D (Variables|Default|GetSFX_Wrong) 1.0 1.0 0.0 0 0))))

(event EventBeginPlay)

(event Collision|EventActorBeginOverlap
  (params (OtherActor :type Actor%20Object%20Reference)))

(event EventTick
  (params (DeltaSeconds :type Float%20%28single-precision%29)))

(fn ConstructionScript)